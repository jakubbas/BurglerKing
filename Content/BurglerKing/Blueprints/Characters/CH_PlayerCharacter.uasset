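; Player character for a loot-stealing game with up to four players, whose ID sets capsule collision channel and spotlight colour.
; Interface events drive movement and relay interact, punch and trap actions to actors overlapping the interaction box.
; Loot is held as data and a mesh, changes walk speed, respawns as a pickup when dropped, and updates the spawner.
; Punches launch and disarm, guards return players to spawn, and power-ups alter speed or collision.
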(event OnComponentBeginOverlap(InteractionBox)
  (params (OverlappedComponent :type Primitive%20Component%20Object%20Reference) (OtherActor :type Actor%20Object%20Reference) (OtherComp :type Primitive%20Component%20Object%20Reference) (OtherBodyIndex :type Integer) (bFromSweep :type Boolean) (SweepResult :type Hit%20Result%20Structure%20%28by%20ref%29))
  ;[0 0.9636 1] Interact box list
  (Utilities|Array|Add (Variables|Default|GetInteractBoxActors) OtherActor))

(event OnComponentEndOverlap(InteractionBox)
  (params (OverlappedComponent :type Primitive%20Component%20Object%20Reference) (OtherActor :type Actor%20Object%20Reference) (OtherComp :type Primitive%20Component%20Object%20Reference) (OtherBodyIndex :type Integer))
  ;[0 0.9636 1] Interact box list
  (Utilities|Array|RemoveItem (Variables|Default|GetInteractBoxActors) OtherActor))

(event Custom|TurnOffSpeed
  (CallFunction|IRemovePowerUp "NewEnumerator0"))

(event Custom|Add%20Trip%20wire%20trap
  (bind _result (Math|Integer|IncrementInt (Variables|Default|GetNumber%20of%20tripWire%20Traps))
    (:%20%20
      (Development|PrintString (Utilities|String|ToString(Integer) _result)))))

(event EventBeginPlay
  (Components|Activation|Deactivate (Variables|Default|GetFollowCamera)))

(event EventIPlayerinSpawn
  (params (PlayerInSpawn :type Boolean))
  (Variables|Default|SetIsInSpawn PlayerInSpawn))

(event EventIMoveForwards
  (params (Direction :type Vector :default "0, 0, 0") (Axis :type Float%20%28double-precision%29))
  ;[0.292 1 0.1971] Axis Movement
  (Pawn|Input|AddMovementInput Direction Axis false))

(event EventIMoveRight
  (params (Direction :type Vector :default "0, 0, 0") (Axis :type Float%20%28double-precision%29))
  ;[0.292 1 0.1971] Axis Movement
  (Pawn|Input|AddMovementInput Direction Axis false))

(event EventIPunchAction
  ;[1 0.5005 0.1834] Input Actions, goes through an array of interactable objects.
  (bind _array_element (Utilities|Array|ForEachLoopwithBreak (Variables|Default|GetInteractBoxActors))
    (:LoopBody
      (Class|BPIPlayerAction|IPunched(Message) _array_element (Transformation|GetActorLocation) self))))

(event EventITrapAction
  ;[1 0.5005 0.1834] Input Actions, goes through an array of interactable objects.
  (bind _array_element (Utilities|Array|ForEachLoopwithBreak (Variables|Default|GetInteractBoxActors))
    (:LoopBody
      (Class|BPIPlayerAction|ITrap(Message) _array_element))))

(event EventIInteractAction
  ;[1 0.5005 0.1834] Input Actions, goes through an array of interactable objects.
  (Utilities|FlowControl|Sequence
    (:then_0
      (bind _array_element (Utilities|Array|ForEachLoopwithBreak (Variables|Default|GetInteractBoxActors))
        (:LoopBody
          (bind _interacttype (Class|BPIPlayerAction|IInteracted(Message) _array_element self))
          (CallFunction|Interact _interacttype _array_element))))
    (:then_1
      ;;[1 1 1] Determines whether the pickup can be dropped or not.
      (if (Variables|Default|GetCanDropItem)
        (CallFunction|DropItem)
        (elif (!= (.name (Variables|Default|GetHeldItem)) "Name")
          (Variables|Default|SetCanDropItem true))))))

(event EventIPlayerCaught
  ;[1 0.02061 0.04051] Player Caught by Guard
  (CallFunction|DropItem)
  (Transformation|SetActorLocation (Transformation|GetActorLocation (Variables|Default|GetSpawner)) false false))

(event EventISetPlayerID
  (params (ID :type Integer))
  (Variables|Default|SetPlayerID ID)
  (CallFunction|SwitchCollisiononID)
  (Class|BPIPlayerHUD|IPlayerID(Message) (UserInterface|GetWidget (Variables|Default|GetPlayerWidget)) (Variables|Default|GetPlayerID))
  (CallFunction|SwitchSpotlightColouronID))

(event EventIPowerUp
  (params (PowerUp :type Enum_PowerUps%20Enum :default "NewEnumerator0"))
  (bind _charactermovement (Variables|Character|GetCharacterMovement))
  (switch Utilities|FlowControl|Switch|SwitchonEnum_PowerUps PowerUp
    (:NewEnumerator0
      ;[0.2131 0.1936 1] Adds on speed to the player.
      (Utilities|Time|SetTimerbyFunctionName 0 "TurnOffSpeed" (Variables|Default|GetSpeedLength))
      (if (not (Utilities|Array|ContainsItem (Variables|Default|GetActivePowerUps) "NewEnumerator0"))
        (Utilities|Array|Add (Variables|Default|GetActivePowerUps) "NewEnumerator0")
        (Variables|/Script/Engine.CharacterMovementComponent|SetMaxWalkSpeed _charactermovement (* (Variables|/Script/Engine.CharacterMovementComponent|GetMaxWalkSpeed _charactermovement) (Variables|Default|GetSpeedMultiplier)))))
    (:NewEnumerator1
      ;[1 0.8675 0.1036] Change the collision channel to pawn.
      (if (not (Utilities|Array|ContainsItem (Variables|Default|GetActivePowerUps) "NewEnumerator1"))
        (Utilities|Array|Add (Variables|Default|GetActivePowerUps) "NewEnumerator1")
        (Collision|SetCollisionObjectType (Variables|Default|GetCapsuleComponent) "ECC_Pawn")))))

(event EventIRemovePowerUp
  (params (PowerUp :type Enum_PowerUps%20Enum :default "NewEnumerator0"))
  (bind _charactermovement (Variables|Character|GetCharacterMovement))
  (switch Utilities|FlowControl|Switch|SwitchonEnum_PowerUps PowerUp
    (:NewEnumerator0
      ;[0.2131 0.1936 1] Removes the added on speed.
      (Variables|/Script/Engine.CharacterMovementComponent|SetMaxWalkSpeed _charactermovement (/ (Variables|/Script/Engine.CharacterMovementComponent|GetMaxWalkSpeed _charactermovement) (Variables|Default|GetSpeedMultiplier)))
      (Utilities|Array|RemoveItem (Variables|Default|GetActivePowerUps) "NewEnumerator0"))
    (:NewEnumerator1
      ;[1 0.8675 0.1036] Change collision channel to the starting one.
      (Collision|SetCollisionObjectType (Variables|Default|GetCapsuleComponent) (Variables|Default|GetCollisionType))
      (Utilities|Array|RemoveItem (Variables|Default|GetActivePowerUps) "NewEnumerator1"))))

(event EventIPunched
  (params (Location :type Vector :default "0, 0, 0") (Instigator :type CH%20Player%20Character%20Object%20Reference))
  (bind _returnvalue (Transformation|GetActorLocation))
  (bind _hitpower (Variables|Default|GetHitPower))
  (bind _returnvalue_2 (Math|Vector|GetUnitDirection(Vector) Location _returnvalue))
  (bind _returnvalue_3 (* _returnvalue_2 _hitpower))
  (bind (_x _y) (Math|Vector|BreakVector _returnvalue_3))
  ;[1 0 0.06238] Player is punched.
  (CallFunction|DropItem)
  (Character|LaunchCharacter (Math|Vector|MakeVector _x _y (Variables|Default|GetHitUpPower)) false false))

(fn ConstructionScript
  (|CallParentFunction))

(fn Interact
  (params (InteractType :type Enum_Interact%20Enum :default "NewEnumerator3") (Actor :type Actor%20Object%20Reference))
  ;[1 0.156 0.9233] Enum switch statement
  (switch Utilities|FlowControl|Switch|SwitchonEnum_Interact InteractType
    (:NewEnumerator0
      (CallFunction|PickUpItem Actor))
    (:NewEnumerator1
      (Variables|Default|SetCanDropItem false))
    (:NewEnumerator2
      (Variables|Default|SetCanDropItem false))))

(fn PickUpItem
  (params (Actor :type Actor%20Object%20Reference))
  (bind _itemmesh (Variables|Default|GetItemMesh))
  ;[0.3708 1 0.3656] Checks if there is already an item in hand.
  (LocalVariables|SetPickUp Actor)
  (if (== (.name (Variables|Default|GetHeldItem)) "Name")
    ;[0.343 1 0.9701] Gets the data from the pickup, saves it and sets new static mesh, then destroys pick up.
    (bind _data (Class|BPIPickUp|IGetDataLoot(Message) (LocalVariables|GetPickUp)))
    (bind _output_get (Variables|Default|SetHeldItem _data))
    (Transformation|SetRelativeScale3D _itemmesh (.scale _output_get))
    (Transformation|SetWorldRotation _itemmesh (.rotation _output_get) false false)
    (Components|StaticMesh|SetStaticMesh _itemmesh (.mesh _output_get))
    (Rendering|Material|SetMaterial _itemmesh 0 (.material _output_get))
    (Class|BPIPickUp|IDestroyPickUp(Message) (LocalVariables|GetPickUp))
    (CallFunction|ChangeSpeed (Variables|Default|GetPlayerSpeedWithItem))
    (if (Variables|Default|GetIsInSpawn)
      (Class|BPISpawn|IContainsLoot(Message) (Variables|Default|GetSpawner) (LocalVariables|GetPickUp)))
    (else
      (Development|PrintString "Already Holding Item"))))

(fn DropItem
  (bind _floorpoint (Variables|Default|GetFloorPoint))
  (bind _floorpoint_2 (Variables|Default|GetFloorPoint))
  (bind _returnvalue (Transformation|GetWorldTransform _floorpoint))
  (bind _returnvalue_2 (Transformation|GetWorldLocation _floorpoint_2))
  ;[1 0.2417 0.7116] Finds the position of the floor infront of the player, and creates the pickup actor there.
  (bind _outhit (Collision|LineTraceByChannel _returnvalue_2 (- _returnvalue_2 "0,0,10000.000000") "TraceTypeQuery1" false 0 "None"))
  (bind _returnvalue_3 (Game|SpawnActorfromClass "/Game/BurglerKing/Blueprints/Environment/Pickups/PickUp_Loot.PickUp_Loot_C" (Math|Transform|MakeTransform (.ImpactPoint (Collision|BreakHitResult _outhit)) (.rotation _returnvalue) (.scale _returnvalue)) "Undefined" 0 0))
  (Variables|/Game/BurglerKing/Blueprints/Environment/Pickups/PickUp_Loot.PickUp_Loot_C|SetIsStolen _returnvalue_3 true)
  (bind _output_get (LocalVariables|SetItem _returnvalue_3))
  ;[0.4816 0.8061 1] Sets the pickup data.
  (Class|BPIPickUp|ISetDataLoot(Message) _output_get (Utilities|Struct|MakeStruct_Loot (.name (Variables|Default|GetHeldItem)) (.price (Variables|Default|GetHeldItem)) (.startlocation (Variables|Default|GetHeldItem)) (.scale (Variables|Default|GetHeldItem)) (Transformation|GetWorldRotation (Variables|Default|GetItemMesh)) (.mesh (Variables|Default|GetHeldItem)) (.material (Variables|Default|GetHeldItem))))
  ;[1 0.9152 0.2937] Resets the static mesh and the required variables to defaults.
  (Transformation|SetWorldRotation (Variables|Default|GetItemMesh) "0, 0, 0" false false)
  (Components|StaticMesh|SetStaticMesh (Variables|Default|GetItemMesh) 0)
  (Variables|Default|SetCanDropItem false)
  (Variables|Default|SetHeldItem (Utilities|Struct|MakeStruct_Loot "Name" 0 "0.000000,0.000000,0.000000" "0.000000,0.000000,0.000000" "0.000000,0.000000,0.000000" 0 0))
  (CallFunction|ChangeSpeed (Variables|Default|GetPlayerSpeed))
  (if (Variables|Default|GetIsInSpawn)
    (Class|BPISpawn|IAddLootinSpawn(Message) (Variables|Default|GetSpawner) (LocalVariables|GetItem))))

(fn SwitchCollisiononID
  (switch int (Variables|Default|GetPlayerID)
    (:0
      (Collision|SetCollisionObjectType (Variables|Default|GetCapsuleComponent) "ECC_GameTraceChannel1")
      (Variables|Default|SetCollisionType "ECC_GameTraceChannel1"))
    (:1
      (Collision|SetCollisionObjectType (Variables|Default|GetCapsuleComponent) "ECC_GameTraceChannel2")
      (Variables|Default|SetCollisionType "ECC_GameTraceChannel2"))
    (:2
      (Collision|SetCollisionObjectType (Variables|Default|GetCapsuleComponent) "ECC_GameTraceChannel3")
      (Variables|Default|SetCollisionType "ECC_GameTraceChannel3"))
    (:3
      (Collision|SetCollisionObjectType (Variables|Default|GetCapsuleComponent) "ECC_GameTraceChannel4")
      (Variables|Default|SetCollisionType "ECC_GameTraceChannel4"))))

(fn SwitchSpotlightColouronID
  (bind _spotlight (Variables|Default|GetSpotLight))
  (bind _spotlight_2 (Variables|Default|GetSpotLight))
  (switch int (Variables|Default|GetPlayerID)
    (:0
      (Rendering|Components|Light|SetLightColor _spotlight_2 "(R=1.000000,G=0.000000,B=0.000000,A=1.000000)" true))
    (:1
      (Rendering|Components|Light|SetLightColor _spotlight_2 "(R=0.000000,G=0.000000,B=1.000000,A=1.000000)" true))
    (:2
      (Rendering|Components|Light|SetLightColor _spotlight "(R=0.000000,G=1.000000,B=0.000000,A=1.000000)" true))
    (:3
      (Rendering|Components|Light|SetLightColor _spotlight "(R=1.000000,G=1.000000,B=0.000000,A=1.000000)" true))))

(fn ChangeSpeed
  (params (NewSpeed :type Float%20%28double-precision%29))
  (Variables|/Script/Engine.CharacterMovementComponent|SetMaxWalkSpeed (Variables|Character|GetCharacterMovement) NewSpeed))

(fn CallPrompt
  (params (Prompt :type Enum_Action%20Enum :default "NewEnumerator0"))
  (Class|BPIPlayerHUD|IPlayerPrompt(Message) (Variables|Default|GetPlayerWidget) Prompt))

(fn DisablePrompt
  (Class|BPIPlayerHUD|ITurnOffPrompt(Message) (Variables|Default|GetPlayerWidget)))

(fn ICheckPlayerinSpawn
  (return (Variables|Default|GetIsInSpawn)))

(fn IGetPlayer
  (return self))

(fn IGetPlayerID
  (return (Variables|Default|GetPlayerID)))

(fn IGetScorefromPlayer
  (bind _score (Class|BPISpawn|IGetScorefromSpawn(Message) (Variables|Default|GetSpawner)))
  (return _score))

(fn IInteracted
  (params (Instigator :type CH%20Player%20Character%20Object%20Reference)))

(fn IReturnType
  (return "NewEnumerator3" 0))