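; Shared multiplayer camera that becomes the first player controller's view target on INITCamera and frames every CH_PlayerCharacter found then.
; Each tick it moves the spring arm to the players' average location and eases its rotation toward that point.
; Arm length eases toward the largest gap between array-adjacent players, scaled and clamped to min/max limits.
; It also counts players within the upper-left 70% of the screen, but never uses the count.
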(event Custom|INIT%20Camera
  (Utilities|FlowControl|Sequence
    (:then_0
      ;[1 1 1] Sets game View to camera
      (bind _asch_player_character (Utilities|Casting|CastToCH_PlayerCharacter (Game|GetPlayerCharacter 0)))
      (Variables|Default|SetPlayer%20Ref _asch_player_character)
      (Game|Player|SetViewTargetwithBlend (Game|GetPlayerController 0) self 0.0 "VTBlend_Linear" 0.0 false))
    (:then_1
      ;[1 1 1] counts the number of active players
      (bind _outactors (Actor|GetAllActorsOfClass "/Game/BurglerKing/Blueprints/Characters/CH_PlayerCharacter.CH_PlayerCharacter_C"))
      (bind _output_get (Variables|Default|SetPlayers _outactors))
      (Variables|Default|SetTotal%20Actors (Math|Conversions|ToFloat(Integer) (Utilities|Array|Length _output_get))))))

(event Custom|Face%20Player
  ;[1 1 1] Face the player
  (bind _returnvalue (Class|GameplayStatics|GetActorArrayAverageLocation (Variables|Default|GetPlayers)))
  (Transformation|SetWorldLocation (Variables|Default|GetSpringArm) _returnvalue false false)
  (Transformation|SetActorRotation (Math|Rotator|MakeRotator 0.0 (Math|Float|ClampAngle (.pitch (Math|Interpolation|RInterpTo (Transformation|GetActorRotation) (Math|Rotator|FindLookatRotation (Transformation|GetActorLocation) _returnvalue) (Utilities|Time|GetWorldDeltaSeconds) 2e+01)) 2e+02 -1.8e+02) (.yaw (Math|Interpolation|RInterpTo (Transformation|GetActorRotation) (Math|Rotator|FindLookatRotation (Transformation|GetActorLocation) _returnvalue) (Utilities|Time|GetWorldDeltaSeconds) 2e+01)))))

(event EventTick
  (params (DeltaSeconds :type Float%20%28single-precision%29))
  (bind _returnvalue (Viewport|GetViewportSize))
  (bind _players (Variables|Default|GetPlayers))
  (bind _springarm (Variables|Default|GetSpringArm))
  (CallFunction|FacePlayer)
  (Utilities|FlowControl|Sequence
    (:then_0
      (Variables|Default|SetSeen%20Actors 0.0)
      (for _array_element (Variables|Default|GetPlayers)
        ;[1 1 1] Finds where abouts on the screen the players are
        (if (Math|Boolean|ANDBoolean (> (.x (.ScreenLocation (Class|PlayerController|ProjectWorldLocationtoScreen (Game|GetPlayerController 0) (Transformation|GetActorLocation _array_element) false))) 0.0) (> (.y (.ScreenLocation (Class|PlayerController|ProjectWorldLocationtoScreen (Game|GetPlayerController 0) (Transformation|GetActorLocation _array_element) false))) 0.0) (< (.x (.ScreenLocation (Class|PlayerController|ProjectWorldLocationtoScreen (Game|GetPlayerController 0) (Transformation|GetActorLocation _array_element) false))) (* (.x _returnvalue) 0.7)) (< (.y (.ScreenLocation (Class|PlayerController|ProjectWorldLocationtoScreen (Game|GetPlayerController 0) (Transformation|GetActorLocation _array_element) false))) (* (.y _returnvalue) 0.7)))
          (Math|Float|IncrementFloat (Variables|Default|GetSeen%20Actors)))))
    (:then_1
      ;[1 1 1] Calculates how many players can be seen and adjust the spring arm
      (Variables|Default|SetLongest%20Distance 0.0)
      (for (_array_element_2 _array_index) _players
        (if (!= _array_index 0)
          (if (> (Transformation|GetDistanceTo _array_element_2 (Utilities|Array|Get(acopy) _players (- _array_index 1))) (Variables|Default|GetLongest%20Distance))
            (Variables|Default|SetLongest%20Distance (Transformation|GetDistanceTo _array_element_2 (Utilities|Array|Get(acopy) _players (- _array_index 1)))))))
      (Variables|Default|SetNew%20Spring%20Arm%20Length (Math|Float|Clamp(Float) (* (Variables|Default|GetLongest%20Distance) 1.2) (Variables|Default|GetMinium%20distance%20away%20from%20the%20player) (Variables|Default|GetMaxium%20distance%20away%20from%20the%20players)))
      (Variables|/Script/Engine.SpringArmComponent|SetTargetArmLength _springarm (Math|Interpolation|FInterpTo (Variables|/Script/Engine.SpringArmComponent|GetTargetArmLength _springarm) (Variables|Default|GetNew%20Spring%20Arm%20Length) (Utilities|Time|GetWorldDeltaSeconds) 1e+01)))))

(fn ConstructionScript)