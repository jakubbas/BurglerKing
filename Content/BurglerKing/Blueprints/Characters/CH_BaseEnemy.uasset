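; Base enemy character that picks a random pig or walrus mesh at BeginPlay and delegates detection and kills to AI_EnemyController.
; An overlap sphere with adjustable radius counts nearby players, enabling the controller's detection only while any are in range.
; KillBox overlaps with a player call KillPlayer on the controller.
; Getters expose vision cone trace settings, patrol checkpoints, movement speeds and the vision widget.
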(event OnComponentBeginOverlap(Sphere)
  (params (OverlappedComponent :type Primitive%20Component%20Object%20Reference) (OtherActor :type Actor%20Object%20Reference) (OtherComp :type Primitive%20Component%20Object%20Reference) (OtherBodyIndex :type Integer) (bFromSweep :type Boolean) (SweepResult :type Hit%20Result%20Structure%20%28by%20ref%29))
  ;[1 0.2054 0.1656] Player Detection Trace Enabler / Disabler Based on players in range.
  (Utilities|Casting|CastToCH_PlayerCharacter OtherActor)
  (Math|Integer|IncrementInt (Variables|Default|GetPlayersInRange)
    (:%20%20
      (CallFunction|SetDetection))))

(event OnComponentEndOverlap(Sphere)
  (params (OverlappedComponent :type Primitive%20Component%20Object%20Reference) (OtherActor :type Actor%20Object%20Reference) (OtherComp :type Primitive%20Component%20Object%20Reference) (OtherBodyIndex :type Integer))
  ;[1 0.2054 0.1656] Player Detection Trace Enabler / Disabler Based on players in range.
  (Utilities|Casting|CastToCH_PlayerCharacter OtherActor)
  (Math|Integer|DecrementInt (Variables|Default|GetPlayersInRange)
    (:%20%20
      (CallFunction|SetDetection))))

(event OnComponentBeginOverlap(KillBox)
  (params (OverlappedComponent :type Primitive%20Component%20Object%20Reference) (OtherActor :type Actor%20Object%20Reference) (OtherComp :type Primitive%20Component%20Object%20Reference) (OtherBodyIndex :type Integer) (bFromSweep :type Boolean) (SweepResult :type Hit%20Result%20Structure%20%28by%20ref%29))
  (bind _asch_player_character (Utilities|Casting|CastToCH_PlayerCharacter OtherActor))
  (bind _asai_enemy_controller (Utilities|Casting|CastToAI_EnemyController (Pawn|GetController)))
  (Default|KillPlayer _asai_enemy_controller _asch_player_character))

(event Custom|SetDetection
  ;[1 0.2054 0.1656] Player Detection Trace Enabler / Disabler Based on players in range.
  (bind _asai_enemy_controller (Utilities|Casting|CastToAI_EnemyController (Pawn|GetController)))
  (if (> (Variables|Default|GetPlayersInRange) 0)
    (Default|EnableDetection _asai_enemy_controller true)
    (else
      (Default|EnableDetection _asai_enemy_controller false))))

(event Custom|SetDetectionSphere
  (params (Sphere%20Radius :type Float%20%28double-precision%29))
  (Components|Sphere|SetSphereRadius (Variables|Default|GetSphere) Sphere%20Radius true)
  (CallFunction|SetDetection))

(event EventBeginPlay
  (bind _mesh (Variables|Character|GetMesh))
  (if (Math|Random|RandomBool)
    (Class|SkinnedMeshComponent|SetSkeletalMesh _mesh "/Game/BurglerKing/Animations/RiggedCharacters/PigRigged.PigRigged" true)
    (else
      (Class|SkinnedMeshComponent|SetSkeletalMesh _mesh "/Game/BurglerKing/Animations/RiggedCharacters/WalrusRigged.WalrusRigged" true))))

(fn ConstructionScript
  (|CallParentFunction))

(fn GetVars
  ;[0 0 0] Get Enemy Variables for Controller
  (return (Variables|Default|GetVision%20Cone%20Length) (Variables|Default|GetVision%20Cone%20Number%20of%20Traces) (Variables|Default|GetVision%20Cone%20Angle)))

(fn GetPatrol
  ;[0 0 0] Return Patrol Variables
  (return (Variables|Default|GetPatrol%20Checkpoints) (Variables|Default|GetPatrol%20Cyclical?)))

(fn GetSpeeds
  ;[0 0 0] Return Speed Variables
  (return (Variables|Default|GetSpeed_Patrol) (Variables|Default|GetSpeed_Chase)))

(fn GetCone
  (return (Variables|Default|GetVisionWidget)))