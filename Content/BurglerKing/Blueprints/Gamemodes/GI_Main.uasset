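; Game instance for BurglerKing that holds shared state: player count, the current music track and player scores keyed by ID.
; Interface events set the player count, store or clear scores, and store and play music as 2D sound, while interface functions return each value.
; Stopping music keeps the stored reference, and the is-playing query only tests whether that reference is set, not actual playback.
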(event EventIStoreandPlayMusicTrack
  (params (Music :type Sound%20Cue%20Object%20Reference))
  (bind _output_get (Variables|Default|SetMusic Music))
  (Audio|PlaySound2D _output_get 0.4 1.0 0.0 0 0))

(event EventIStorePlayerScores
  (params (IDsAndPlayers :type Map%20of%20Integers%20to%20Integers))
  (Variables|Default|SetIDs%20and%20Scores IDsAndPlayers))

(event EventISetPlayerCount
  (params (PlayerCount :type Integer))
  (Variables|Default|SetPlayerCount PlayerCount))

(event EventIClearScores
  (Utilities|Map|Clear (Variables|Default|GetIDs%20and%20Scores)))

(event EventIStopCurrentMusicTrack
  (Class|AudioLinkBlueprintInterface|StopLink(Message) (Variables|Default|GetMusic)))

(fn IGetMusicTrack
  (return (Variables|Default|GetMusic)))

(fn IGetPlayerCount
  (return (Variables|Default|GetPlayerCount)))

(fn IGetPlayerScores
  (return (Variables|Default|GetIDs%20and%20Scores)))

(fn IIsPlayingMusicTrack
  (return (!= (Variables|Default|GetMusic) 0)))