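; Post-game game mode for BurglerKing that shows the end screen with player scores ranked highest first.
; On BeginPlay it creates the UI_EndScreen widget and switches to UI-only input with a visible cursor.
; It then pulls the ID-to-score map from the game instance through an interface message, selection-sorts it by repeatedly moving the top entry into a temp map, and passes the result to the widget.
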(event Custom|UpdateScores
  (bind _idsandplayers (Class|BPIGameInstance|IGetPlayerScores(Message) (Game|GetGameInstance)))
  (Variables|Default|SetIDsAndScores _idsandplayers)
  (CallFunction|SortScores)
  (Default|ChangeScores (Variables|Default|GetEndScreen) (Variables|Default|GetIDsAndScores)))

(event EventBeginPlay
  (bind _returnvalue (Game|GetPlayerController 0))
  (bind _returnvalue_2 (UserInterface|CreateWidget "/Game/BurglerKing/w027457k/Widgets/UI_EndScreen.UI_EndScreen_C" (Game|GetPlayerController 0)))
  (bind _output_get (Variables|Default|SetEndScreen _returnvalue_2))
  (UserInterface|Viewport|AddtoViewport _output_get 0)
  (Input|SetInputModeUIOnly _returnvalue _returnvalue_2 "DoNotLock")
  (Variables|/Script/Engine.PlayerController|SetbShowMouseCursor _returnvalue true)
  (CallFunction|UpdateScores))

(fn ConstructionScript)

(fn SortScores
  ;[0.3642 1 0.9801] While the length of the array isn't 0.
  (while (Utilities|Map|IsNotEmpty (Variables|Default|GetIDsAndScores))
    ;[1 0.2889 0.6661] Add the best value out of integer array to temp array, and remove it from integer array.
    (bind _values (Utilities|Map|Values (Variables|Default|GetIDsAndScores)))
    (bind _keys (Utilities|Map|Keys (Variables|Default|GetIDsAndScores)))
    (Utilities|Map|Add (LocalVariables|GetTempMap) (Utilities|Array|Get(acopy) _keys (.IndexOfMaxValue (Math|Integer|MaxOfIntArray _values))) (.MaxValue (Math|Integer|MaxOfIntArray _values)))
    (Utilities|Map|Remove (Variables|Default|GetIDsAndScores) (Utilities|Array|Get(acopy) _keys (.IndexOfMaxValue (Math|Integer|MaxOfIntArray _values)))))
  ;[0.9098 1 0.1232] Set the sorted array.
  (Variables|Default|SetIDsAndScores (LocalVariables|GetTempMap)))