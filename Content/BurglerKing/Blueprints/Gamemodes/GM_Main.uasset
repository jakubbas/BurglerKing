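; Main game mode for BurglerKing that sets up a two-player local session.
; BeginPlay runs Init, which creates the local players, then calls PreGame; the PreGame, InGame and PostGame phase events are empty stubs.
; Each new player gets a CH_BaseCharacter at a fixed location, possessed and announced through ISetPawnMessage.
; Login and logout maintain the Controllers list, while batch spawning and extra-player removal helpers sit unwired.
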(event Custom|Init
  (CallFunction|SetUpControllers 2)
  (CallFunction|PreGame))

(event Custom|PreGame)

(event Custom|InGame)

(event Custom|PostGame)

(event EventBeginPlay
  (CallFunction|Init))

(event EventOnLogout
  (params (ExitingController :type Controller%20Object%20Reference))
  (Utilities|Array|RemoveItem (Variables|Default|GetControllers) ExitingController))

(event EventPostLogin
  (params (NewPlayer :type Player%20Controller%20Object%20Reference))
  (Utilities|Array|Add (Variables|Default|GetControllers) NewPlayer))

(event EventHandleStartingNewPlayer
  (params (NewPlayer :type Player%20Controller%20Object%20Reference))
  (bind _returnvalue (Game|SpawnActorfromClass "/Game/BurglerKing/Blueprints/Characters/CH_BaseCharacter.CH_BaseCharacter_C" (Math|Transform|MakeTransform "100.000000,110.000000,1250.000000" "0, 0, 0" "1.000000,1.000000,1.000000") "Undefined" 0 0))
  (Pawn|Possess NewPlayer _returnvalue)
  (Class|BPIPlayerController|ISetPawn(Message) NewPlayer _returnvalue))

(fn ConstructionScript)

(fn SetUpControllers
  (params (Player :type Integer))
  (Variables|Default|SetPlayerCount Player)
  (for _index (range 0 (- Player 1))
    (Class|GameplayStatics|CreatePlayer _index)))

(fn RemoveOtherPlayers
  (for _index (range 1 (- (Variables|Default|GetPlayerCount) 1))
    (Utilities|IsValid (Class|GameplayStatics|GetPlayerControllerfromID _index)
      (:Is%20Valid
        (Class|GameplayStatics|RemovePlayer (Class|GameplayStatics|GetPlayerControllerfromID _index) true)))))

(fn SpawnCharacters
  (for _array_element (Variables|Default|GetControllers)
    (bind _returnvalue (Game|SpawnActorfromClass "/Game/BurglerKing/Blueprints/Characters/CH_BaseCharacter.CH_BaseCharacter_C" (Math|Transform|MakeTransform "90.000000,1100.000000,100.000000" "0, 0, 0" "1.000000,1.000000,1.000000") "Undefined" 0 0))
    (Utilities|Array|Add (Variables|Default|GetCharacters) _returnvalue)
    (Pawn|Possess _array_element _returnvalue)
    (Class|BPIPlayerController|ISetPawn(Message) _array_element _returnvalue)
    (Development|PrintString (Utilities|GetDisplayName _returnvalue))))