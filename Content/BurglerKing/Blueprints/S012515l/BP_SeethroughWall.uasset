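; A trigger-box Blueprint that turns a set of referenced wall meshes see-through while something overlaps its box.
; On overlap begin, it creates dynamic instances of the entry material on each wall, and a timeline drives their GridOpacity parameter.
; On overlap end, a second timeline plays in reverse on those instances, then restores the exit material and clears the instance array.
; Older fade logic remains in the graph, disconnected.
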(event OnComponentEndOverlap(Box)
  (params (OverlappedComponent :type Primitive%20Component%20Object%20Reference) (OtherActor :type Actor%20Object%20Reference) (OtherComp :type Primitive%20Component%20Object%20Reference) (OtherBodyIndex :type Integer))
  (if (Utilities|Array|IsNotEmpty (Variables|Default|GetDynamicMaterial))
    (bind _newtrack_0 (Timeline|ChangeOpacityReverse ReverseFromEnd)
      (:Update
        (for _array_element (Variables|Default|GetDynamicMaterial)
          (Rendering|Material|SetScalarParameterValue _array_element "GridOpacity" _newtrack_0 :!class /Script/Engine.MaterialInstanceDynamic)))
      (:Finished
        (for _array_element_2 (Variables|Default|GetWalls)
          (Rendering|Material|SetMaterial (Variables|/Script/Engine.StaticMeshActor|GetStaticMeshComponent _array_element_2) 0 (Variables|Default|GetMaterial%20on%20exit))
          (Utilities|Array|Clear (Variables|Default|GetDynamicMaterial)))))))

(event OnComponentBeginOverlap(Box)
  (params (OverlappedComponent :type Primitive%20Component%20Object%20Reference) (OtherActor :type Actor%20Object%20Reference) (OtherComp :type Primitive%20Component%20Object%20Reference) (OtherBodyIndex :type Integer) (bFromSweep :type Boolean) (SweepResult :type Hit%20Result%20Structure%20%28by%20ref%29))
  (for _array_element (Variables|Default|GetWalls)
    (bind _returnvalue (Rendering|Material|CreateDynamicMaterialInstance (Variables|/Script/Engine.StaticMeshActor|GetStaticMeshComponent _array_element) 0 (Variables|Default|GetMaterial%20on%20entry) "None" :!class /Script/Engine.PrimitiveComponent))
    (Utilities|Array|Add (Variables|Default|GetDynamicMaterial) _returnvalue))
  (bind _newtrack_0 (Timeline|ChangeOpacity PlayFromStart)
    (:Update
      (for _array_element_2 (Variables|Default|GetDynamicMaterial)
        (Rendering|Material|SetScalarParameterValue _array_element_2 "GridOpacity" _newtrack_0 :!class /Script/Engine.MaterialInstanceDynamic)))))

(fn ConstructionScript)