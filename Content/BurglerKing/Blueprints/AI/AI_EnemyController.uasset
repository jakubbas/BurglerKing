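; AI controller for enemy guards that detects players, noises and stolen loot, feeding BT_EnemyAI through its blackboard.
; Player sight uses a custom cone: recursive line traces sweep the pawn's yaw, repeating via a timeline that can be toggled.
; Visible players are mapped by distance; the closest sets target and last-known position, clearing any sound position.
; Perception components report noise locations and stolen loot; pawn variables configure the cone, detection sphere and patrol/chase speeds.
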(event OnTargetPerceptionUpdated(SightPerceiver)
  (params (Actor :type Actor%20Object%20Reference) (Stimulus :type AI%20Stimulus%20Structure))
  ;[0 0 0] Perceive Sight (Used to find stolen loot)
  (bind _aspick_up_loot (Utilities|Casting|CastToPickUp_Loot Actor))
  (bind _isstolen (Class|BPIPickUp|IIsLootStolen(Message) _aspick_up_loot))
  (if _isstolen
    (AI|Components|Blackboard|SetValueasObject (Variables|Default|GetBB) (Utilities|Name|MakeLiteralName "DroppedLootPos") _aspick_up_loot)))

(event OnTargetPerceptionUpdated(AudioPerceiver)
  (params (Actor :type Actor%20Object%20Reference) (Stimulus :type AI%20Stimulus%20Structure))
  ;[0 0 0] Percieve Noises
  (AI|Components|Blackboard|SetValueasVector (Variables|Default|GetBB) (Utilities|Name|MakeLiteralName "SoundPos") (.stimuluslocation Stimulus)))

(event Custom|Set%20Variables
  (params (TraceLength :type Float%20%28double-precision%29) (NumberOfTraces :type Integer) (ConeAngle :type Float%20%28double-precision%29))
  ;[0 0 0] Init
  ;;[0 0 0] Set Vision Cone Variables
  (Variables|Default|SetTrace%20Length TraceLength)
  (Variables|Default|SetNumberOfTraces NumberOfTraces)
  (Variables|Default|SetCone%20Angle ConeAngle))

(event Custom|SetTraceVariables
  (bind _returnvalue (Pawn|GetControlledPawn))
  ;[0 0 0] Player Detection
  ;;[1 0.5183 0.6915] Set Trace Variables
  (Variables|Default|SetPawn%20Location (Transformation|GetActorLocation _returnvalue))
  ;;;[0 0 0] Start Angle = Z Rotation - 1/2(Cone Angle) Traces can then iterate from here +X each time
  (Variables|Default|SetPawn%20Rotation (Transformation|GetActorRotation _returnvalue))
  (Variables|Default|SetStartAngle (- (.yaw (Variables|Default|GetPawn%20Rotation)) (/ (Variables|Default|GetCone%20Angle) 2.0))))

(event Custom|Set%20Detection%20Sphere
  ;[0 0 0] Init
  ;;[0 0 0] Sets the player detection distance requirement equal to trace distance + 100
  (Default|SetDetectionSphere (Variables|Default|GetControlledPawn) (+ (Variables|Default|GetTrace%20Length) 1e+02)))

(event Custom|SetActorsToIgnore
  ;[0 0 0] Init
  ;;[1 0.3383 0.2785] Find actors of classes to ignore
  (for _array_element (Variables|Default|GetIgnoredClasses)
    (bind _outactors (Actor|GetAllActorsOfClass _array_element))
    (for _array_element_2 _outactors
      (Utilities|Array|Add (Variables|Default|GetActors%20to%20Ignore) _array_element_2))))

(event Custom|TraceForPlayer
  ;[0 0 0] Player Detection
  ;;[1 0.267 0] Trace For Player
  (if (< (Variables|Default|GetTrace%20Number) (Variables|Default|GetNumberOfTraces))
    (CallFunction|CalculateTraceIteration (Variables|Default|GetTrace%20Number))
    ;;;[0 0 0] Trace / Cast to player
    (bind _outhit (Collision|LineTraceForObjects (Variables|Default|GetPawn%20Location) (+ (Variables|Default|GetPawn%20Location) (* (Math|Vector|GetForwardVector (Variables|Default|GetTrace%20Rotation)) (Variables|Default|GetTrace%20Length))) (Variables|Default|GetObject%20Types) false (Variables|Default|GetActors%20to%20Ignore) "ForDuration" true "(R=0.000000,G=1.000000,B=0.094117,A=1.000000)" "(R=0.395833,G=0.024279,B=0.016403,A=1.000000)" 0.1))
    (bind _asch_player_character (Utilities|Casting|CastToCH_PlayerCharacter (.hitactor _outhit))
      (:then
        (CallFunction|StorePlayerInfo _asch_player_character (.distance _outhit))
        (if (Utilities|Array|ContainsItem (Variables|Default|GetHitPlayers) _asch_player_character)
          _
          (else
            (Utilities|Array|Add (Variables|Default|GetHitPlayers) _asch_player_character))))
      (:CastFailed
        _))
    (Math|Integer|IncrementInt (Variables|Default|GetTrace%20Number)
      (:%20%20
        (CallFunction|TraceforPlayer)))
    (else
      ;;;[0 0 0] Once the trace is complete, call the reset / set trace number back to 0
      (Variables|Default|SetTrace%20Number 0)
      (CallFunction|FindClosestPlayer)
      (CallFunction|TraceCooldown))))

(event Custom|TraceCooldown
  ;[0 0 0] Player Detection
  ;;[0 0.2963 1] Reset Trace for player | Remove players from visible list if they weren't detected in previous trace
  (if (Utilities|Array|IsNotEmpty (Variables|Default|GetHitPlayers))
    (bind _keys (Utilities|Map|Keys (Variables|Default|GetVisiblePlayers)))
    (for _array_element _keys
      (if (not (Utilities|Array|ContainsItem (Variables|Default|GetHitPlayers) _array_element))
        (Utilities|Map|Remove (Variables|Default|GetVisiblePlayers) _array_element)))
    (else
      (Utilities|Map|Clear (Variables|Default|GetVisiblePlayers))
      (AI|Components|Blackboard|SetValueasObject (Variables|Default|GetBB) (Variables|Default|GetClosestPlayerKey) 0)))
  (Utilities|Array|Clear (Variables|Default|GetHitPlayers))
  (Timeline|TraceRestartTimeline PlayFromStart
    (:Finished
      (CallFunction|SetTraceVariables)
      (CallFunction|TraceforPlayer))))

(event Custom|Calculate%20Trace%20Iteration
  (params (Iteration :type Integer))
  (bind _pawn_rotation (Variables|Default|GetPawn%20Rotation))
  ;[0 0 0] Player Detection
  ;;[0.4181 0.5565 1] Calculate Trace Angle From Iteration
  ;;;[0 0 0] Trace angle = Start Angle + Iteration(Cone Angle / Number of Traces)
  (Variables|Default|SetTrace%20Rotation (Math|Rotator|MakeRotator (.roll _pawn_rotation) (.pitch _pawn_rotation) (+ (Variables|Default|GetStartAngle) (* Iteration (/ (Variables|Default|GetCone%20Angle) (Variables|Default|GetNumberOfTraces)))))))

(event Custom|StorePlayerInfo
  (params (Pawn%20Detected :type Pawn%20Object%20Reference) (Distance :type Float%20%28double-precision%29))
  ;[0 0 0] Player Detection
  ;;[0.02352 0.474 0.2787] Handle Player Trace Data
  ;;;[0 0 0] Add Player Pawn Ref + Distance from guard to map
  (Utilities|Map|Add (Variables|Default|GetVisiblePlayers) Pawn%20Detected Distance))

(event Custom|Init
  (params (Trace%20Length :type Float%20%28double-precision%29) (Number%20of%20Traces :type Integer) (Cone%20Angle :type Float%20%28double-precision%29))
  ;[0 0 0] Init
  ;;[1 0.8968 0.4463] Init Chain
  (CallFunction|SetVariables Trace%20Length Number%20of%20Traces Cone%20Angle)
  (AI|RunBehaviorTree "/Game/BurglerKing/Blueprints/AI/BT_EnemyAI.BT_EnemyAI")
  (bind _blackboardcomponent (Class|AIController|UseBlackboard "/Game/BurglerKing/Blueprints/AI/BB_EnemyAI.BB_EnemyAI"))
  (bind _output_get (Variables|Default|SetBB _blackboardcomponent))
  (AI|Components|Blackboard|SetValueasBool _output_get (Utilities|Name|MakeLiteralName "Forwards") true)
  (CallFunction|SetActorstoIgnore)
  (Utilities|Array|Add (Variables|Default|GetActors%20to%20Ignore) (Pawn|GetControlledPawn))
  (CallFunction|SetTraceVariables)
  (CallFunction|TraceforPlayer)
  (CallFunction|SetDetectionSphere))

(event Custom|Find%20Closest%20Player
  (bind _bb (Variables|Default|GetBB))
  ;[0 0 0] Player Detection
  ;;[0.02352 0.474 0.2787] Handle Player Trace Data
  ;;;[0 0 0] Find Closest Player
  (Variables|Default|SetClosest%20Player 0)
  (Variables|Default|SetClosest%20Distance 999999.0)
  (bind _keys (Utilities|Map|Keys (Variables|Default|GetVisiblePlayers)))
  (for _array_element _keys
    (if (< (.Value (Utilities|Map|Find (Variables|Default|GetVisiblePlayers) _array_element)) (Variables|Default|GetClosest%20Distance))
      (Variables|Default|SetClosest%20Distance (.Value (Utilities|Map|Find (Variables|Default|GetVisiblePlayers) _array_element)))
      (Variables|Default|SetClosest%20Player _array_element)))
  ;;;[0 0 0] Store Closest Player + Their location in the Blackboard
  (Utilities|IsValid (Variables|Default|GetClosest%20Player)
    (:Is%20Valid
      (AI|Components|Blackboard|SetValueasObject _bb (Variables|Default|GetClosestPlayerKey) (Variables|Default|GetClosest%20Player))
      (AI|Components|Blackboard|SetValueasVector _bb (Variables|Default|GetLastKnownPosKey) (Transformation|GetActorLocation (Variables|Default|GetClosest%20Player)))
      (AI|Components|Blackboard|ClearValue _bb (Utilities|Name|MakeLiteralName "SoundPos")))))

(event Custom|Set%20Speed
  (params (Chasing? :type Boolean))
  (bind _controlledpawn (Variables|Default|GetControlledPawn))
  (bind _charactermovement (Variables|/Script/Engine.Character|GetCharacterMovement _controlledpawn))
  ;[1 0.09705 0.8588] Set Speed
  (bind (_speedpatrol _speedchase) (Default|GetSpeeds _controlledpawn))
  (if Chasing?
    (Variables|/Script/Engine.CharacterMovementComponent|SetMaxWalkSpeed _charactermovement _speedchase)
    (else
      (Variables|/Script/Engine.CharacterMovementComponent|SetMaxWalkSpeed _charactermovement _speedpatrol))))

(event Custom|Enable%20Detection
  (params (Enabled? :type Boolean))
  ;[0 0 0] Player Detection
  ;;[0 0.2963 1] Reset Trace for player | Remove players from visible list if they weren't detected in previous trace
  ;;;[0 0 0] Disables Player Detection Tracing when no players are near
  (if Enabled?
    (Timeline|TraceRestartTimeline Play
      (:Finished
        (CallFunction|SetTraceVariables)
        (CallFunction|TraceforPlayer)))
    (else
      (Timeline|TraceRestartTimeline Stop))))

(event EventBeginPlay
  ;[0 0 0] Init
  ;;[0 0 0] Get pawn / call Init
  (bind _asch_base_enemy (Utilities|Casting|CastToCH_BaseEnemy (Pawn|GetControlledPawn)))
  (bind _output_get (Variables|Default|SetControlledPawn _asch_base_enemy))
  (bind (_trace_length _trace_number _cone_angle) (Default|GetVars _output_get))
  (CallFunction|Init _trace_length _trace_number _cone_angle))

(fn ConstructionScript)

(fn Trace
  (params (Iteration1 :type Integer)))