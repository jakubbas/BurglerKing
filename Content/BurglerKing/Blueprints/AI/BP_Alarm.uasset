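; BP_Alarm is an AI alarm actor that alerts by emitting noise and flashing a spotlight when triggered.
; An interface Activate event reports noise at the actor's location with a configurable range, attributed to the instigator, then shows the SpotLight for five seconds before hiding it.
; An older collision-based trigger that ignored enemy pawns remains in the graph, disconnected and marked redundant.
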(event Custom|Make%20Noise
  (params (Max%20Range :type Float%20%28double-precision%29) (Instigator :type Pawn%20Object%20Reference))
  (bind _self self)
  ;[0 0 0] Make Noise
  (Class|Actor|MakeNoise _self 1.0 Instigator (Transformation|GetActorLocation _self) Max%20Range "None"))

(event EventActivate
  (params (Instigator :type CH%20Player%20Character%20Object%20Reference))
  ;[0.9007 0.6813 1] Activate Via Interface
  (CallFunction|MakeNoise (Variables|Default|GetMax%20Range) Instigator)
  (Rendering|SetVisibility (Variables|Default|GetSpotLight) true false)
  (Utilities|FlowControl|Delay 5.0)
  (Rendering|SetVisibility (Variables|Default|GetSpotLight) false false))

(fn ConstructionScript)