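; BP_Door is an environment double door that other objects drive through Activate and Deactivate events.
; BeginPlay derives mirrored yaw targets for the left and right sockets from OpenAngle, and DoorTimeline lerps between them, reversing to close.
; Normally Activate closes and Deactivate opens.
; With ConstantState, Activate is ignored and Deactivate toggles through a FlipFlop, which DefaultState triggers at BeginPlay to start the door opening.
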(event Custom|Open%20Door
  ;[0.125 0.03492 0.04114] Door Opening
  (bind _floattrack (Timeline|DoorTimeline Play)
    (:Update
      (Transformation|SetWorldRotation (Variables|Default|GetLeftSocket) (Math|Rotator|Lerp(Rotator) (Variables|Default|GetStartRotLeft) (Variables|Default|GetEndRotLeft) _floattrack) false false)
      (Transformation|SetWorldRotation (Variables|Default|GetRightSocket) (Math|Rotator|Lerp(Rotator) (Variables|Default|GetStartRotRight) (Variables|Default|GetEndRotRight) _floattrack) false false))))

(event Custom|Close%20Door
  ;[0.125 0.03492 0.04114] Door Opening
  (bind _floattrack (Timeline|DoorTimeline Reverse)
    (:Update
      (Transformation|SetWorldRotation (Variables|Default|GetLeftSocket) (Math|Rotator|Lerp(Rotator) (Variables|Default|GetStartRotLeft) (Variables|Default|GetEndRotLeft) _floattrack) false false)
      (Transformation|SetWorldRotation (Variables|Default|GetRightSocket) (Math|Rotator|Lerp(Rotator) (Variables|Default|GetStartRotRight) (Variables|Default|GetEndRotRight) _floattrack) false false))))

(event Custom|ToggleDoor
  ;[0 0 0] Toggles Door State
  (Utilities|FlowControl|FlipFlop
    (:A
      (CallFunction|OpenDoor))
    (:B
      (CallFunction|CloseDoor))))

(event EventBeginPlay
  ;[0.7671 0.6063 0.8281] Set Variables
  (bind _output_get (Variables|Default|SetStartRotLeft (Transformation|GetWorldRotation (Variables|Default|GetLeftSocket))))
  (Variables|Default|SetEndRotLeft (Math|Rotator|MakeRotator (.roll _output_get) (.pitch _output_get) (+ (.yaw _output_get) (Variables|Default|GetOpenAngle))))
  (bind _output_get_2 (Variables|Default|SetStartRotRight (Transformation|GetWorldRotation (Variables|Default|GetRightSocket))))
  (Variables|Default|SetEndRotRight (Math|Rotator|MakeRotator (.roll _output_get_2) (.pitch _output_get_2) (- (.yaw _output_get_2) (Variables|Default|GetOpenAngle))))
  (if (Variables|Default|GetConstantState?)
    (if (Variables|Default|GetDefaultState)
      (CallFunction|ToggleDoor))))

(event EventDeactivate
  ;[0 0 0] Activate throuh interface
  (if (Variables|Default|GetConstantState?)
    (CallFunction|ToggleDoor)
    (else
      (CallFunction|OpenDoor))))

(event EventActivate
  (params (Instigator :type CH%20Player%20Character%20Object%20Reference))
  ;[0 0 0] Activate throuh interface
  (if (not (Variables|Default|GetConstantState?))
    (CallFunction|CloseDoor)))

(fn ConstructionScript)