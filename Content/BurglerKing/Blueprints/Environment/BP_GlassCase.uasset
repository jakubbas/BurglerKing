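; BP_GlassCase is a breakable display case that keeps its Loot out of reach by disabling that mesh's collision at BeginPlay.
; The first punch received through the IPunched interface event destroys the placeholder glass mesh and re-enables loot collision.
; The break also plays a shatter sound and calls MakeNoise with the puncher as instigator, limited to ShatterNoiseRange.
; Both interaction interface functions return one fixed enum value.
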(event OnAudioFinished(ShatterNoise)
  ;[0 0 0] MAKE NOISE
  (Audio|Components|Audio|Stop (Variables|Default|GetShatterNoise)))

(event Custom|BreakGlass
  ;[1 0 0] Break the glass mesh, for now this just destroys the placeholder cube
  (Components|DestroyComponent (Variables|Default|GetStaticMesh)))

(event Custom|Make%20Loot%20Interactable
  ;[1 0 0] Make Loot Interactable
  (Collision|SetCollisionEnabled (Variables|/Game/BurglerKing/Blueprints/Environment/Pickups/BP_PickUp.BP_PickUp_C|GetStaticMesh (Variables|Default|GetLoot)) "QueryAndPhysics"))

(event Custom|CreateNoise
  (params (Instigator :type CH%20Player%20Character%20Object%20Reference) (Location :type Vector))
  ;[0 0 0] MAKE NOISE
  (Class|Actor|MakeNoise 1.0 Instigator Location (Variables|Default|GetShatter%20Noise%20Range) "None")
  (Audio|Components|Audio|Play (Variables|Default|GetShatterNoise) 0.0))

(event EventBeginPlay
  ;[1 0 0] Make Loot Interactable
  ;;[0 0 0] Prevent Interaction on Spawn
  (Collision|SetCollisionEnabled (Variables|/Game/BurglerKing/Blueprints/Environment/Pickups/BP_PickUp.BP_PickUp_C|GetStaticMesh (Variables|Default|GetLoot)) "NoCollision"))

(event EventIPunched
  (params (Location :type Vector :default "0, 0, 0") (Instigator :type CH%20Player%20Character%20Object%20Reference))
  ;[0 0 0] Punch recieved via interface
  (Utilities|FlowControl|DoOnce false
    (:Completed
      (CallFunction|BreakGlass)
      (CallFunction|MakeLootInteractable)
      (CallFunction|CreateNoise Instigator Location))))

(fn ConstructionScript)

(fn IInteracted
  (params (Instigator :type CH%20Player%20Character%20Object%20Reference))
  (return "NewEnumerator3"))

(fn IReturnType
  (return "NewEnumerator3" 0))