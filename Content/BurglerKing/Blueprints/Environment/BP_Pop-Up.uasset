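; BP_Pop-Up is a world actor that shows a one-time text pop-up when something overlaps its sphere.
; On BeginPlay it sizes its widget component, passes its text to the UI_Pop-Up widget and hides it.
; The first sphere overlap, from any actor, makes the widget visible through a DoOnce, then hides it again after a configurable delay without destroying the actor.
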(event OnComponentBeginOverlap(Sphere)
  (params (OverlappedComponent :type Primitive%20Component%20Object%20Reference) (OtherActor :type Actor%20Object%20Reference) (OtherComp :type Primitive%20Component%20Object%20Reference) (OtherBodyIndex :type Integer) (bFromSweep :type Boolean) (SweepResult :type Hit%20Result%20Structure%20%28by%20ref%29))
  (Utilities|FlowControl|DoOnce false
    (:Completed
      (CallFunction|EnablePop-Up true)
      (CallFunction|Despawn))))

(event Custom|Init
  (bind _popup_widget (Variables|Default|GetPopUp_Widget))
  ;[1 0.8119 0.6784] Init chain
  (Class|WidgetComponent|SetDrawSize _popup_widget (Math|Vector2D|MakeVector2D (Variables|Default|GetWidth) (Variables|Default|GetHeight)))
  (bind _asui_pop__up (Utilities|Casting|CastToUI_Pop-Up (UserInterface|GetUserWidgetObject _popup_widget)))
  (Default|ChangeText _asui_pop__up (Variables|Default|GetText)))

(event Custom|Enable%20Pop-Up
  (params (Enable? :type Boolean))
  ;[0 0 0] Toggle widget visibility
  (Rendering|SetVisibility (Variables|Default|GetPopUp_Widget) Enable? false))

(event Custom|Despawn
  ;[0 0 0] Remove Widget
  (Utilities|FlowControl|Delay (Variables|Default|GetDe-spawn%20Delay))
  (CallFunction|EnablePop-Up false))

(event EventBeginPlay
  (CallFunction|Init)
  (CallFunction|EnablePop-Up false))

(fn ConstructionScript)