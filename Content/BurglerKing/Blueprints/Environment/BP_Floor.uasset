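; BP_Floor is a configurable floor piece for the environment, built on a Plane component.
; Its construction script creates a dynamic material instance from SourceMaterial on the plane's first material slot and stores it in MaterialInstance.
; It then pushes the actor's U and V tiling and Color variables into the material parameters, so each placed floor can have its own look.
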(fn ConstructionScript
  (bind _returnvalue (Rendering|Material|CreateDynamicMaterialInstance (Variables|Default|GetPlane) 0 (Variables|Default|GetSource%20Material) "None" :!class /Script/Engine.PrimitiveComponent))
  (bind _output_get (Variables|Default|SetMaterialInstance _returnvalue))
  (Rendering|Material|SetScalarParameterValue _output_get "UTiling" (Variables|Default|GetUTiling) :!class /Script/Engine.MaterialInstanceDynamic)
  (Rendering|Material|SetScalarParameterValue (Variables|Default|GetMaterialInstance) "VTiling" (Variables|Default|GetVTiling) :!class /Script/Engine.MaterialInstanceDynamic)
  (Rendering|Material|SetVectorParameterValue (Variables|Default|GetMaterialInstance) "Color" (Variables|Default|GetColor) :!class /Script/Engine.MaterialInstanceDynamic))