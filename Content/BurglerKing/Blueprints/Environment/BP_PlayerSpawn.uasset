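; Per-player spawn base that banks dropped loot and scores it for its owner.
; Loot added or removed re-sums item prices and reports to the GameMode, while DetectionBox overlaps notify actors of being inside.
; The spawn ID sets the light color and which player collision channel BarrierBox ignores; non-owners leaving that box lose a specific power-up.
; A timed disable raises blocking boxes and a visible mesh, then re-enables the spawn.
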(event OnComponentBeginOverlap(DetectionBox)
  (params (OverlappedComponent :type Primitive%20Component%20Object%20Reference) (OtherActor :type Actor%20Object%20Reference) (OtherComp :type Primitive%20Component%20Object%20Reference) (OtherBodyIndex :type Integer) (bFromSweep :type Boolean) (SweepResult :type Hit%20Result%20Structure%20%28by%20ref%29))
  ;[0.4464 0.8173 1] Tells the player if they're inside the spawn.
  (Class|BPIPlayer|IPlayerinSpawn(Message) OtherActor true))

(event OnComponentEndOverlap(DetectionBox)
  (params (OverlappedComponent :type Primitive%20Component%20Object%20Reference) (OtherActor :type Actor%20Object%20Reference) (OtherComp :type Primitive%20Component%20Object%20Reference) (OtherBodyIndex :type Integer))
  ;[1 0.9946 0.2389] If the list contains the exiting item, remove it.
  (if (Utilities|Array|ContainsItem (Variables|Default|GetCurrentLoot) OtherActor)
    (Utilities|Array|RemoveItem (Variables|Default|GetCurrentLoot) OtherActor)
    (CallFunction|UpdateScore)
    (else
      (Class|BPIPlayer|IPlayerinSpawn(Message) OtherActor false))))

(event OnComponentEndOverlap(BarrierBox)
  (params (OverlappedComponent :type Primitive%20Component%20Object%20Reference) (OtherActor :type Actor%20Object%20Reference) (OtherComp :type Primitive%20Component%20Object%20Reference) (OtherBodyIndex :type Integer))
  (bind _id (Class|BPIPlayer|IGetPlayerID(Message) OtherActor))
  (if (!= _id (Variables|Default|GetPlayerSpawnID))
    (Class|BPIPlayer|IRemovePowerUp(Message) OtherActor "NewEnumerator1")))

(event Custom|UpdateScore
  ;[1 0.3366 0.001466] Anytime the loot array is updated, this gets a new score value and updates the gamemode.
  (for _array_element (Variables|Default|GetCurrentLoot)
    (bind _data (Class|BPIPickUp|IGetDataLoot(Message) _array_element))
    (Variables|Default|SetTempScore (+ (Variables|Default|GetTempScore) (.Price (Utilities|Struct|BreakStruct_Loot _data)))))
  (Development|PrintString (Utilities|String|ToString(Integer) (Variables|Default|GetTempScore)))
  (Variables|Default|SetCurrentScore (Variables|Default|GetTempScore))
  (Variables|Default|SetTempScore 0)
  (CallFunction|UpdateGamemode))

(event Custom|EnableSpawn
  ;[1 0.2344 0.2344] Enable/Disable Spawn
  (Collision|SetCollisionEnabled (Variables|Default|GetBlockBox) "NoCollision")
  (Rendering|SetVisibility (Variables|Default|GetBlockMesh) false false))

(event EventIUpdateSpawnerID
  (params (ID :type Integer))
  ;[0.7994 1 0.519] Switches the collision response to the player channels based on the spawn id.
  (bind _output_get (Variables|Default|SetPlayerSpawnID ID))
  (switch int _output_get
    (:0
      (Collision|SetCollisionResponsetoChannel (Variables|Default|GetBarrierBox) "ECC_GameTraceChannel1" "ECR_Ignore")
      (Rendering|Components|Light|SetLightColor (Variables|Default|GetRectLight) "(R=1.000000,G=0.000000,B=0.000000,A=1.000000)" true))
    (:1
      (Collision|SetCollisionResponsetoChannel (Variables|Default|GetBarrierBox) "ECC_GameTraceChannel2" "ECR_Ignore")
      (Rendering|Components|Light|SetLightColor (Variables|Default|GetRectLight) "(R=0.000000,G=0.000000,B=1.000000,A=1.000000)" true))
    (:2
      (Collision|SetCollisionResponsetoChannel (Variables|Default|GetBarrierBox) "ECC_GameTraceChannel3" "ECR_Ignore")
      (Rendering|Components|Light|SetLightColor (Variables|Default|GetRectLight) "(R=0.000000,G=1.000000,B=0.000000,A=1.000000)" true))
    (:3
      (Collision|SetCollisionResponsetoChannel (Variables|Default|GetBarrierBox) "ECC_GameTraceChannel4" "ECR_Ignore")
      (Rendering|Components|Light|SetLightColor (Variables|Default|GetRectLight) "(R=1.000000,G=1.000000,B=0.000000,A=1.000000)" true))))

(event EventIAddLootinSpawn
  (params (Loot :type Actor%20Object%20Reference))
  ;[0.07245 1 0.1129] Player dropped loot in the spawn, adds it to the array.
  (Utilities|Array|Add (Variables|Default|GetCurrentLoot) Loot)
  (CallFunction|UpdateScore)
  (Class|BPIGM|IUpdateRemainingLootAmountGM(Message) (Game|GetGameMode) -1))

(event EventIContainsLoot
  (params (Loot :type Actor%20Object%20Reference))
  ;[1 0.3037 0.7555] If the current loot array has the new picked up loot by the player, it will remove it from the list.
  (if (Utilities|Array|ContainsItem (Variables|Default|GetCurrentLoot) Loot)
    (Utilities|Array|RemoveItem (Variables|Default|GetCurrentLoot) Loot)
    (CallFunction|UpdateScore)
    (Class|BPIGM|IUpdateRemainingLootAmountGM(Message) (Game|GetGameMode) 1)))

(event EventIDisableSpawn
  (params (Time :type Float%20%28double-precision%29))
  ;[1 0.2344 0.2344] Enable/Disable Spawn
  (Utilities|Time|SetTimerbyFunctionName 0 "EnableSpawn" Time)
  (Collision|SetCollisionEnabled (Variables|Default|GetBlockBox) "QueryAndPhysics")
  (Rendering|SetVisibility (Variables|Default|GetBlockMesh) true false))

(event EventBeginPlay
  (Collision|SetCollisionEnabled (Variables|Default|GetBlockBox) "NoCollision")
  (Rendering|SetVisibility (Variables|Default|GetBlockMesh) false false))

(fn ConstructionScript
  (Rendering|SetVisibility (Variables|Default|GetBlockMesh) false false)
  (Transformation|SetRelativeScale3D (Variables|Default|GetBarrierBox) (Variables|Default|GetOutsideBoxSize)))

(fn UpdateGamemode
  (Class|BPIGamemodeUI|IUpdateScore(Message) (Game|GetGameMode) (Variables|Default|GetPlayerSpawnID) (Variables|Default|GetCurrentScore)))

(fn SwitchSpawnColouronID
  (switch int (Variables|Default|GetPlayerSpawnID)
    (:0
      (Rendering|Components|Light|SetLightColor (Variables|Default|GetRectLight) "(R=1.000000,G=0.000000,B=0.000000,A=1.000000)" true))
    (:1
      (Rendering|Components|Light|SetLightColor (Variables|Default|GetRectLight) "(R=0.000000,G=0.000000,B=1.000000,A=1.000000)" true))
    (:2
      (Rendering|Components|Light|SetLightColor (Variables|Default|GetRectLight) "(R=0.000000,G=1.000000,B=0.000000,A=1.000000)" true))
    (:3
      (Rendering|Components|Light|SetLightColor (Variables|Default|GetRectLight) "(R=1.000000,G=1.000000,B=0.000000,A=1.000000)" true))))

(fn IGetScorefromSpawn
  (return (Variables|Default|GetCurrentScore)))