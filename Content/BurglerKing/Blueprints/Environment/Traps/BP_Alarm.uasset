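; Alarm trap that, when activated through an interface, alerts AI with noise attributed to its instigator until a guard arrives.
; Activation lights a spotlight, plays alarm audio and starts a self-restarting timeline that repeats MakeNoise on each finish, with a DoOnce guarding the one-shot cue.
; An enemy overlapping the box turns off the light and audio, stops the loop and re-arms the trap.
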(event OnComponentBeginOverlap(Box)
  (params (OverlappedComponent :type Primitive%20Component%20Object%20Reference) (OtherActor :type Actor%20Object%20Reference) (OtherComp :type Primitive%20Component%20Object%20Reference) (OtherBodyIndex :type Integer) (bFromSweep :type Boolean) (SweepResult :type Hit%20Result%20Structure%20%28by%20ref%29))
  ;[1 0.1406 0.1406] Reset alarm when guard arrives
  (Utilities|Casting|CastToCH_BaseEnemy OtherActor)
  (Rendering|SetVisibility (Variables|Default|GetSpotLight) false false)
  (Variables|Default|SetReady? true)
  (CallFunction|StopAlarm)
  (Audio|Components|Audio|Stop (Variables|Default|GetAlarm%20Noise)))

(event Custom|Make%20Noise
  (params (Max%20Range :type Float%20%28double-precision%29) (Instigator :type Pawn%20Object%20Reference))
  (bind _self self)
  ;[0 0 0] Make Noise
  (Class|Actor|MakeNoise _self 1.0 Instigator (Transformation|GetActorLocation _self) Max%20Range "None"))

(event Custom|StartAlarm
  (Utilities|FlowControl|Sequence
    (:then_0
      (Utilities|FlowControl|DoOnce false
        (:Completed
          (Audio|PlaySoundatLocation "/Game/BurglerKing/Assets/Sounds/SE_AlarmCue.SE_AlarmCue" (Transformation|GetActorLocation) "0, 0, 0" 0.6 1.0 0.0 0 0 0 0))))
    (:then_1
      (Timeline|Alarm%20Timeline PlayFromStart
        (:Finished
          (CallFunction|MakeNoise (Variables|Default|GetMax%20Range) (Variables|Default|GetPlayerInstigator))
          (CallFunction|StartAlarm))))))

(event Custom|StopAlarm
  (Utilities|FlowControl|Sequence
    (:then_0
      (Utilities|FlowControl|DoOnce false) ; enters at Reset
    )
    (:then_1
      (Timeline|Alarm%20Timeline Stop
        (:Finished
          (CallFunction|MakeNoise (Variables|Default|GetMax%20Range) (Variables|Default|GetPlayerInstigator))
          (CallFunction|StartAlarm))))))

(event EventActivate
  (params (Instigator :type CH%20Player%20Character%20Object%20Reference))
  ;[0.9007 0.6813 1] Activate Via Interface
  (if (Variables|Default|GetReady?)
    (bind _output_get (Variables|Default|SetPlayerInstigator Instigator))
    (CallFunction|MakeNoise (Variables|Default|GetMax%20Range) _output_get)
    (Rendering|SetVisibility (Variables|Default|GetSpotLight) true false)
    (CallFunction|StartAlarm)
    (Variables|Default|SetReady? false)
    (Audio|Components|Audio|Play (Variables|Default|GetAlarm%20Noise) 0.0)))

(fn ConstructionScript)