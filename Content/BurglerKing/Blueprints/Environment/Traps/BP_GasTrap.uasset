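; Gas trap hazard that runs a Niagara gas cloud and starts respawn timers for players inside its area.
; Activate is gated by a DoOnce, which Deactivate resets after a delay as it switches the cloud off.
; Overlap events track players in an array alongside a parallel array of timer handles, clearing a player's timer on exit.
; Timers start on activation for players already inside, or on entry while active.
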(event OnComponentBeginOverlap(GasArea_0)
  (params (OverlappedComponent :type Primitive%20Component%20Object%20Reference) (OtherActor :type Actor%20Object%20Reference) (OtherComp :type Primitive%20Component%20Object%20Reference) (OtherBodyIndex :type Integer) (bFromSweep :type Boolean) (SweepResult :type Hit%20Result%20Structure%20%28by%20ref%29))
  (bind _player_array (Variables|Default|GetPlayer%20array))
  (bind _asch_player_character (Utilities|Casting|CastToCH_PlayerCharacter OtherActor))
  (if (not (Utilities|Array|ContainsItem _player_array _asch_player_character))
    (Utilities|Array|AddUnique _player_array _asch_player_character)
    (if (Variables|Default|GetIsActive?)
      (bind _returnvalue (Utilities|Time|SetTimerbyEvent (EventDispatchers|CreateEvent _asch_player_character :!event IPlayerCaught) 2.0))
      (Utilities|Array|Add (Variables|Default|GetRespawn%20Timer%20Array) _returnvalue))))

(event OnComponentEndOverlap(GasArea_0)
  (params (OverlappedComponent :type Primitive%20Component%20Object%20Reference) (OtherActor :type Actor%20Object%20Reference) (OtherComp :type Primitive%20Component%20Object%20Reference) (OtherBodyIndex :type Integer))
  (bind _respawn_timer_array (Variables|Default|GetRespawn%20Timer%20Array))
  (bind _asch_player_character (Utilities|Casting|CastToCH_PlayerCharacter OtherActor))
  (Utilities|Time|ClearandInvalidateTimerbyHandle (Utilities|Array|Get(acopy) _respawn_timer_array (Utilities|Array|FindItem (Variables|Default|GetPlayer%20array) _asch_player_character)))
  (Utilities|Array|RemoveItem _respawn_timer_array (Utilities|Array|Get(acopy) _respawn_timer_array (Utilities|Array|FindItem (Variables|Default|GetPlayer%20array) _asch_player_character)))
  (Utilities|Array|RemoveItem (Variables|Default|GetPlayer%20array) _asch_player_character))

(event EventActivate
  (params (Instigator :type CH%20Player%20Character%20Object%20Reference))
  (Utilities|FlowControl|DoOnce false
    (:Completed
      (Variables|Default|SetIsActive? true)
      (Components|Activation|Activate (Variables|Default|GetNS_GasCloud) true)
      (for _array_element (Variables|Default|GetPlayer%20array)
        (bind _returnvalue (Utilities|Time|SetTimerbyEvent (EventDispatchers|CreateEvent _array_element :!event IPlayerCaught) 2.0))
        (Utilities|Array|Add (Variables|Default|GetRespawn%20Timer%20Array) _returnvalue)))))

(event EventDeactivate
  (bind _ns_gascloud (Variables|Default|GetNS_GasCloud))
  (Utilities|FlowControl|Delay 6.0)
  (Utilities|FlowControl|Sequence
    (:then_0
      (Variables|Default|SetIsActive? false)
      (Components|Activation|Deactivate _ns_gascloud)
      (Utilities|Time|ClearandInvalidateTimerbyHandle (Variables|Default|GetTimer%20Ref)))
    (:then_1
      (Utilities|FlowControl|DoOnce false) ; enters at Reset
    )))

(fn ConstructionScript)

(fn IReturnType
  (return "NewEnumerator3" 0))

(fn IInteracted
  (return "NewEnumerator3"))

(fn ICheckPlayerinSpawn
  (return false))

(fn IGetPlayer
  (return 0))

(fn IGetScorefromPlayer
  (return 0))