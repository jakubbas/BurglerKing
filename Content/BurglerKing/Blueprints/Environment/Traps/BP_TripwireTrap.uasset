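; Tripwire trap actor that stuns characters who walk into it and can be disabled by players.
; Its hit box arms after two seconds; the first valid overlap snaps the cable and zeroes walk speed for StunDuration.
; A second overlap volume enables input and opens a gate, so holding Interact for MaxHoldTime breaks the trap.
; Breaking destroys the hit box and calls AddTrap, intended to credit a player with a tripwire.
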(event OnComponentEndOverlap(HitBox)
  (params (OverlappedComponent :type Primitive%20Component%20Object%20Reference) (OtherActor :type Actor%20Object%20Reference) (OtherComp :type Primitive%20Component%20Object%20Reference) (OtherBodyIndex :type Integer))
  ;[1 1 1] Stuns player when they walk into trap
  (Utilities|FlowControl|DoOnce false) ; enters at Reset
)

(event OnComponentBeginOverlap(HitBox)
  (params (OverlappedComponent :type Primitive%20Component%20Object%20Reference) (OtherActor :type Actor%20Object%20Reference) (OtherComp :type Primitive%20Component%20Object%20Reference) (OtherBodyIndex :type Integer) (bFromSweep :type Boolean) (SweepResult :type Hit%20Result%20Structure%20%28by%20ref%29))
  (bind _returnvalue (Actor|GetComponentbyClass OtherActor "/Script/Engine.CharacterMovementComponent"))
  ;[1 1 1] Stuns player when they walk into trap
  (if (not (Variables|Default|GetIsBroken?))
    (Utilities|FlowControl|DoOnce false
      (:Completed
        (Utilities|IsValid _returnvalue
          (:Is%20Valid
            (Rendering|SetVisibility (Variables|Default|GetbrokenCableL) true false)
            (Rendering|SetVisibility (Variables|Default|GetCable) false false)
            (Variables|Default|SetIsBroken? true)
            (Variables|Default|SetMax%20Walk%20Speed (Variables|/Script/Engine.CharacterMovementComponent|GetMaxWalkSpeed _returnvalue))
            (Variables|/Script/Engine.CharacterMovementComponent|SetMaxWalkSpeed _returnvalue 0.0)
            (Utilities|FlowControl|Delay (Variables|Default|GetStun%20duration))
            (Variables|/Script/Engine.CharacterMovementComponent|SetMaxWalkSpeed _returnvalue (Variables|Default|GetMax%20Walk%20Speed))))))))

(event OnComponentBeginOverlap(DisabletrapOverlap)
  (params (OverlappedComponent :type Primitive%20Component%20Object%20Reference) (OtherActor :type Actor%20Object%20Reference) (OtherComp :type Primitive%20Component%20Object%20Reference) (OtherBodyIndex :type Integer) (bFromSweep :type Boolean) (SweepResult :type Hit%20Result%20Structure%20%28by%20ref%29))
  ;[1 1 1] Checks if players are in the overlap area
  (Utilities|Casting|CastToCH_PlayerCharacter OtherActor)
  (Input|EnableInput (Game|GetPlayerController 0))
  (Utilities|FlowControl|Gate true) ; enters at Open
)

(event OnComponentEndOverlap(DisabletrapOverlap)
  (params (OverlappedComponent :type Primitive%20Component%20Object%20Reference) (OtherActor :type Actor%20Object%20Reference) (OtherComp :type Primitive%20Component%20Object%20Reference) (OtherBodyIndex :type Integer))
  ;[1 1 1] Checks if players are in the overlap area
  (Utilities|Casting|CastToCH_PlayerCharacter OtherActor)
  (Input|DisableInput (Game|GetPlayerController 0))
  (Utilities|FlowControl|Gate true) ; enters at Close
)

(event Custom|Timer
  ;[1 1 1] Timer on how long it takes for player to break trap
  (bind _returnvalue (Utilities|Time|SetTimerbyEvent (delegate Custom|Timer) (Variables|Default|GetMax%20hold%20time))))

(event Custom|Stop%20Timer
  ;[1 1 1] Timer on how long it takes for player to break trap
  (Utilities|Time|PauseTimerbyHandle (stale Custom|Timer _returnvalue)))

(event Custom|Update%20Timer
  ;[1 1 1] Timer on how long it takes for player to break trap
  (if (Variables|Default|GetIsHeld?)
    (Utilities|FlowControl|Delay 0.1)
    (CallFunction|UpdateTimer)
    (else
      (CallFunction|StopTimer))))

(event Custom|Break%20Tripwire
  ;[1 1 1] Stuns player when they walk into trap
  ;;[1 1 1] Breaks trap when players interact with trap
  (Rendering|SetVisibility (Variables|Default|GetbrokenCableL) true false)
  (Rendering|SetVisibility (Variables|Default|GetCable) false false)
  (Variables|Default|SetIsBroken? true)
  (Components|DestroyComponent (Variables|Default|GetHitBox)))

(event Custom|Turn%20On%20Trap
  ;[1 1 1] Sets the initial visibilty of the cable
  (Collision|SetCollisionEnabled (Variables|Default|GetHitBox) "QueryOnly"))

(event Custom|Add%20Trap
  (params (Player%20Ref :type CH%20Player%20Character%20Object%20Reference))
  ;[1 1 1] Checks if players are in the overlap area
  (Default|AddTripWireTrap Player%20Ref))

(event EventBeginPlay
  ;[1 1 1] Sets the initial visibilty of the cable
  (Utilities|Time|SetTimerbyEvent (delegate Custom|Turn%20On%20Trap) 2.0)
  (Rendering|SetVisibility (Variables|Default|GetbrokenCableL) false false))

(event Input|ActionEvents|InputActionInteract
  (params (Key :type Key%20Structure :default "None"))
  ;[1 1 1] Checks if players are in the overlap area
  (:Pressed
    (Variables|Default|SetIsHeld? true)
    (Utilities|FlowControl|Gate true
      (:Exit
        (Utilities|FlowControl|Sequence
          (:then_0
            (Utilities|FlowControl|RetriggerableDelay (Variables|Default|GetMax%20hold%20time))
            (if (Variables|Default|GetIsHeld?)
              (CallFunction|BreakTripwire)
              (CallFunction|AddTrap)))
          (:then_1
            (CallFunction|Timer)
            (CallFunction|UpdateTimer))))))
  (:Released
    (Variables|Default|SetIsHeld? false)))

(fn ConstructionScript)

(fn IReturnType
  (return "NewEnumerator3" 0))

(fn IInteracted
  (params (Instigator :type CH%20Player%20Character%20Object%20Reference))
  (return "NewEnumerator3"))