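; BP_FloorTrap is a pressure plate that triggers linked traps when the player character steps on its box.
; A DoOnce gate plays a cue sound and sends an activate message with the player to every TrapRef entry.
; After a Cooldown delay, it re-arms and sends deactivate only to the loop's last element.
; It also answers interaction interface queries with fixed enum values.
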(event OnComponentBeginOverlap(Box)
  (params (OverlappedComponent :type Primitive%20Component%20Object%20Reference) (OtherActor :type Actor%20Object%20Reference) (OtherComp :type Primitive%20Component%20Object%20Reference) (OtherBodyIndex :type Integer) (bFromSweep :type Boolean) (SweepResult :type Hit%20Result%20Structure%20%28by%20ref%29))
  (bind _asch_player_character (Utilities|Casting|CastToCH_PlayerCharacter OtherActor))
  (Class|BPIPlayer|IGetPlayer(Message) OtherActor)
  (Utilities|FlowControl|DoOnce false
    (:Completed
      (Audio|PlaySoundatLocation "/Game/BurglerKing/Assets/Sounds/SE_PressurePlateCue.SE_PressurePlateCue" (Transformation|GetActorLocation) "0, 0, 0" 1.0 1.0 0.0 0 0 0 0)
      (Actor|GetAllActorswithInterface "/Game/BurglerKing/Blueprints/Interfaces/BPI_PlayerAction.BPI_PlayerAction_C")
      (for _array_element (Variables|Default|GetTrap%20Ref)
        (Class|BPITrap|Activate(Message) _array_element _asch_player_character))
      (Utilities|FlowControl|Delay (Variables|Default|Getcooldown))
      (CallFunction|TrapReset)
      (Class|BPITrap|Deactivate(Message) _array_element))))

(event Custom|TrapReset
  (Utilities|FlowControl|DoOnce false) ; enters at Reset
)

(fn ConstructionScript)

(fn IInteracted
  (params (Instigator :type CH%20Player%20Character%20Object%20Reference))
  (return "NewEnumerator3"))

(fn IReturnType
  (return "NewEnumerator3" "NewEnumerator7" 0))