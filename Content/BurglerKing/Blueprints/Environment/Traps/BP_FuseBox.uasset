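; Interactable fuse box trap object that temporarily switches off its linked Output actors.
; Interacting while Ready clears the flag and sends DeactivateMessage to every Output, then starts a reset delay.
; After the delay it sends ActivateMessage to the Outputs and sets Ready again.
; The reactivation event also calls the reset event, so the delayed ActivateMessage repeats after the first use.
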(event Custom|FuseBoxActivated
  ;[0 0 0] Activation
  (for _array_element (Variables|Default|GetOutputs)
    (Class|BPITrap|Deactivate(Message) _array_element))
  (CallFunction|ResetFuseBox))

(event Custom|ResetFuseBox
  ;[0 0 0] Reset After Delay
  (Utilities|FlowControl|Delay (Variables|Default|GetReset%20Delay))
  (CallFunction|FuseBoxDeactivated)
  (Variables|Default|SetReady? true))

(event Custom|FuseBoxDeactivated
  ;[0 0 0] Deactivation
  (for _array_element (Variables|Default|GetOutputs)
    (Class|BPITrap|Activate(Message) _array_element))
  (CallFunction|ResetFuseBox))

(fn ConstructionScript)

(fn IInteracted
  (params (Instigator :type CH%20Player%20Character%20Object%20Reference))
  (if (Variables|Default|GetReady?)
    (Variables|Default|SetReady? false)
    (CallFunction|FuseBoxActivated)
    (return "NewEnumerator3")))

(fn IReturnType
  (return "NewEnumerator1" "NewEnumerator1" self))