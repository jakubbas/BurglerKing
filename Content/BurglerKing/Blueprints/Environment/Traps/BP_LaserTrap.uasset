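; BP_LaserTrap is a laser tripwire trap that signals linked objects when the player crosses it.
; A Box overlap by CH_PlayerCharacter sends ActivateMessage with that character to each entry in Outputs, then disables the laser.
; SetLaser toggles beam visibility and box collision together.
; Disable is temporary, restoring the laser after ResetTime even when triggered by the external Deactivate event, while Activate switches it on.
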(event OnComponentBeginOverlap(Box)
  (params (OverlappedComponent :type Primitive%20Component%20Object%20Reference) (OtherActor :type Actor%20Object%20Reference) (OtherComp :type Primitive%20Component%20Object%20Reference) (OtherBodyIndex :type Integer) (bFromSweep :type Boolean) (SweepResult :type Hit%20Result%20Structure%20%28by%20ref%29))
  ;[1 0.3785 0.901] Laser Activation From Collision
  (bind _asch_player_character (Utilities|Casting|CastToCH_PlayerCharacter OtherActor))
  (for _array_element (Variables|Default|GetOutputs)
    (Class|BPITrap|Activate(Message) _array_element _asch_player_character))
  (CallFunction|Disable))

(event Custom|SetLaser
  (params (Enabled? :type Boolean))
  (bind _laser (Variables|Default|GetLaser))
  ;[1 0.2899 0.1297] Disable / Reset Laser
  (if Enabled?
    (Rendering|SetVisibility _laser true false)
    (Collision|SetCollisionEnabled (Variables|Default|GetBox) "QueryAndPhysics")
    (else
      (Rendering|SetVisibility _laser false false)
      (Collision|SetCollisionEnabled (Variables|Default|GetBox) "NoCollision"))))

(event Custom|Disable
  ;[1 0.2899 0.1297] Disable / Reset Laser
  (CallFunction|SetLaser false)
  (Utilities|FlowControl|Delay (Variables|Default|GetReset%20Time))
  (CallFunction|SetLaser true))

(event Custom|Enable
  ;[1 0.2899 0.1297] Disable / Reset Laser
  (CallFunction|SetLaser true))

(event EventDeactivate
  (CallFunction|Disable))

(event EventActivate
  (params (Instigator :type CH%20Player%20Character%20Object%20Reference))
  (CallFunction|Enable))

(fn ConstructionScript)