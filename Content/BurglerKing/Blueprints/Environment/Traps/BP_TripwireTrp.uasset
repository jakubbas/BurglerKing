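; Tripwire trap that snaps when a character walks into it, briefly halting them.
; The first hit box overlap by an actor with a CharacterMovementComponent swaps the intact cable for two broken halves and sets IsBroken, so it triggers once.
; It zeroes the victim's walk speed, then restores it after a short delay; fall and get-up animations are unconnected placeholders.
; Interaction interface functions return a fixed enum value.
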(event OnComponentEndOverlap(HitBox)
  (params (OverlappedComponent :type Primitive%20Component%20Object%20Reference) (OtherActor :type Actor%20Object%20Reference) (OtherComp :type Primitive%20Component%20Object%20Reference) (OtherBodyIndex :type Integer))
  (Utilities|FlowControl|DoOnce false) ; enters at Reset
)

(event OnComponentBeginOverlap(HitBox)
  (params (OverlappedComponent :type Primitive%20Component%20Object%20Reference) (OtherActor :type Actor%20Object%20Reference) (OtherComp :type Primitive%20Component%20Object%20Reference) (OtherBodyIndex :type Integer) (bFromSweep :type Boolean) (SweepResult :type Hit%20Result%20Structure%20%28by%20ref%29))
  (bind _returnvalue (Actor|GetComponentbyClass OtherActor "/Script/Engine.CharacterMovementComponent"))
  (if (not (Variables|Default|GetIsBroken?))
    (Utilities|FlowControl|DoOnce false
      (:Completed
        (Utilities|IsValid _returnvalue
          (:Is%20Valid
            (Rendering|SetVisibility (Variables|Default|GetbrokenCableL) true false)
            (Rendering|SetVisibility (Variables|Default|GetCable) false false)
            (Development|PrintString "broken state")
            (Variables|Default|SetIsBroken? true)
            (Variables|Default|SetMax%20Walk%20Speed (Variables|/Script/Engine.CharacterMovementComponent|GetMaxWalkSpeed _returnvalue))
            (Variables|/Script/Engine.CharacterMovementComponent|SetMaxWalkSpeed _returnvalue 0.0)
            (Utilities|FlowControl|Delay 0.5)
            (Variables|/Script/Engine.CharacterMovementComponent|SetMaxWalkSpeed _returnvalue (Variables|Default|GetMax%20Walk%20Speed))))))))

(event EventBeginPlay
  (Rendering|SetVisibility (Variables|Default|GetbrokenCableL) false false))

(fn ConstructionScript)

(fn IReturnType
  (return "NewEnumerator3" 0))

(fn IInteracted
  (params (Instigator :type CH%20Player%20Character%20Object%20Reference))
  (return "NewEnumerator3"))